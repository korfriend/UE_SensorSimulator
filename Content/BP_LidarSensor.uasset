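; BP_LidarSensor is an actor that simulates a lidar sensor with a scene capture camera and a point cloud component.
; BeginPlay creates the camera's render target and an empty point cloud optimized for dynamic data.
; Each Tick starts an async scan using both components and a fixed field of view, storing the result via delegate.
; An event can swap in an external render target, releasing the internally created one.
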(event Custom|MyTestDelegate_Event
  (params (SensorOut :type Lidar%20Sensor%20Out%20Structure))
  (Variables|Default|SetLidarSensorOut SensorOut))

(event Custom|SetRenderTarget_Event
  (params (RenderTargetTexture :type Texture%20Render%20Target%202D%20Object%20Reference))
  (if (Variables|Default|GetIsInitialized)
    (if (== RenderTargetTexture (Variables|Default|GetCameraRenderTarget))
      _
      (elif (Variables|Default|GetIsIntrinsicRenderTarget)
        (Class|KismetRenderingLibrary|ReleaseRenderTarget2D (Variables|Default|GetCameraRenderTarget))))
    (bind _output_get (Variables|Default|SetCameraRenderTarget RenderTargetTexture))
    (Variables|/Script/Engine.SceneCaptureComponent2D|SetTextureTarget (Variables|Default|GetCamera) _output_get)))

(event Collision|EventActorBeginOverlap
  (params (OtherActor :type Actor%20Object%20Reference)))

(event EventTick
  (params (DeltaSeconds :type Float%20%28single-precision%29))
  (if (Variables|Default|GetIsInitialized)
    (Class|SensorSimulatorBPLibrary|LidarSensorAsyncScan4 (Variables|Default|GetLidarPointsArray) (Variables|Default|GetPC_Lidar) (Variables|Default|GetCamera) (delegate Custom|MyTestDelegate_Event) true -15.0 35.0 (Variables|Default|GetLidarChannels) 1.5e+02 (Variables|Default|GetLidarRes) 1e+03)))

(event EventBeginPlay
  (bind _pc_lidar (Variables|Default|GetPC_Lidar))
  (Utilities|FlowControl|Sequence
    (:then_0
      (bind _returnvalue (Rendering|CreateRenderTarget2D (Variables|Default|GetCaptureImageWidth) (Variables|Default|GetCaptureImageHeight) "RTF_RGBA8"))
      (bind _output_get (Variables|Default|SetCameraRenderTarget _returnvalue))
      (Variables|/Script/Engine.SceneCaptureComponent2D|SetTextureTarget (Variables|Default|GetCamera) _output_get)
      (Variables|Default|SetIsIntrinsicRenderTarget true))
    (:then_1
      (Class|LidarPointCloudComponent|SetPointCloud _pc_lidar (Class|LidarPointCloudBlueprintLibrary|CreatePointCloudEmpty))
      (Class|LidarPointCloud|SetOptimizedforDynamicData (Variables|/Script/LidarPointCloudRuntime.LidarPointCloudComponent|GetPointCloud _pc_lidar) true)
      (Variables|Default|SetIsInitialized true))))

(fn ConstructionScript)